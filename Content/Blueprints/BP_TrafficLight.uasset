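; Traffic light actor with red, yellow and green lamps that light up according to its current color state.
; BeginPlay gives each lamp its own dynamic instance of a shared color material.
; ChangeColor switches on CurrentColor, applies the passed color to that lamp and blacks out only its predecessor, assuming a green, yellow, red cycle.
; CurrentColor is never set in this graph.
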(event `self.ReceiveBeginPlay`
  ;[1 1 1] Create basic materials for lamps
  (bind _returnvalue (`PrimitiveComponent.CreateDynamicMaterialInstance` (`self.GreenLamp`) 0 "/Game/Blueprints/Materials/M_TrafficColorInstance.M_TrafficColorInstance" "None"))
  (set `self.GreenMaterial` _returnvalue)
  (bind _returnvalue_2 (`PrimitiveComponent.CreateDynamicMaterialInstance` (`self.YellowLamp`) 0 "/Game/Blueprints/Materials/M_TrafficColorInstance.M_TrafficColorInstance" "None"))
  (set `self.YellowMaterial` _returnvalue_2)
  (bind _returnvalue_3 (`PrimitiveComponent.CreateDynamicMaterialInstance` (`self.RedLamp`) 0 "/Game/Blueprints/Materials/M_TrafficColorInstance.M_TrafficColorInstance" "None"))
  (set `self.RedMaterial` _returnvalue_3))

(event `ChangeColor`
  (params (Color :type "LinearColor Structure"))
  ;[1 1 1] Sets new color for traffic light
  (switch `/Game/Blueprints/E_LightColor` (`self.CurrentColor`)
    (:`NewEnumerator0`
      (`MaterialInstanceDynamic.SetVectorParameterValue` (`self.RedMaterial`) "Color" Color)
      (`MaterialInstanceDynamic.SetVectorParameterValue` :`self` (`self.YellowMaterial`) :`ParameterName` "Color"))
    (:`NewEnumerator1`
      (`MaterialInstanceDynamic.SetVectorParameterValue` (`self.YellowMaterial`) "Color" Color)
      (`MaterialInstanceDynamic.SetVectorParameterValue` :`self` (`self.GreenMaterial`) :`ParameterName` "Color"))
    (:`NewEnumerator2`
      (`MaterialInstanceDynamic.SetVectorParameterValue` (`self.GreenMaterial`) "Color" Color)
      (`MaterialInstanceDynamic.SetVectorParameterValue` :`self` (`self.RedMaterial`) :`ParameterName` "Color"))))

(fn `UserConstructionScript`)