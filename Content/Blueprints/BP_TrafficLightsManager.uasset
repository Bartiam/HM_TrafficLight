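; BP_TrafficLightsManager cycles the color of all BP_TrafficLight actors in the level on a timer.
; After a short BeginPlay delay to let lamps and lights spawn, it gathers the lights and calls Recolor.
; Recolor applies each light's current color from the ColorSettings map, then advances its state from red to green to yellow and back.
; Each Recolor call re-sets a looping timer by function name to repeat itself.
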(event `self.ReceiveBeginPlay`
  ;[1 1 1] Delay for creating lamps and traffic lights
  (`KismetSystemLibrary.Delay` 0.2)
  ;[1 1 1] Gets all traffic lights
  (bind _outactors (`GameplayStatics.GetAllActorsOfClass` "/Game/Blueprints/BP_TrafficLight.BP_TrafficLight_C"))
  (set `self.TrafficLights` _outactors)
  (`self.Recolor`))

(fn `Recolor`
  (locals (CurrentTrafficLight :type "/Game/Blueprints/BP_TrafficLight Object Reference"))
  (bind _colorsettings_colormap (break `/Game/Blueprints/S_LIghtColor` (`self.ColorSettings`)))
  (for _array_element (`self.TrafficLights`)
    (bind _output_get (set `local.CurrentTrafficLight` _array_element))
    (`/Game/Blueprints/BP_TrafficLight.ChangeColor` _output_get (`BlueprintMapLibrary.Map_Find` _colorsettings_colormap (`/Game/Blueprints/BP_TrafficLight.CurrentColor` _array_element)))
    (switch `/Game/Blueprints/E_LightColor` (`/Game/Blueprints/BP_TrafficLight.CurrentColor` (`local.CurrentTrafficLight`))
      (:`NewEnumerator0`
        (set `/Game/Blueprints/BP_TrafficLight.CurrentColor` "NewEnumerator2" (`local.CurrentTrafficLight`)))
      (:`NewEnumerator1`
        (set `/Game/Blueprints/BP_TrafficLight.CurrentColor` "NewEnumerator0" (`local.CurrentTrafficLight`)))
      (:`NewEnumerator2`
        (set `/Game/Blueprints/BP_TrafficLight.CurrentColor` "NewEnumerator1" (`local.CurrentTrafficLight`)))))
  (`KismetSystemLibrary.K2_SetTimer` null "Recolor" 2.0 true))

(fn `UserConstructionScript`)